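; MenuMode sets up the start menu level on BeginPlay, likely as its game mode, swapping in the pawn for the play kind stored in MenuGameInstance.
; It spawns a VR or third-person menu pawn at a player start, destroys the current pawn and possesses the new one.
; It then spawns a scaled 3D StartMenuActor in front of the player, attaches it to the pawn and stores its WB_Menu widget as StartMenu.
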(event EventBeginPlay
  (bind _returnvalue (Game|GetPlayerController 0))
  (bind _returnvalue_2 (Class|GameModeBase|FindPlayerStart _returnvalue "None"))
  (bind _returnvalue_3 (Transformation|GetActorTransform _returnvalue_2))
  (bind _asmenu_game_instance (Utilities|Casting|CastToMenuGameInstance (Game|GetGameInstance)))
  (switch Utilities|FlowControl|Switch|SwitchonEPlayKind (Variables|/Game/Menu/Blueprints/MenuGameInstance.MenuGameInstance_C|GetPlayKind _asmenu_game_instance)
    (:NewEnumerator0
      (bind _returnvalue_4 (Game|SpawnActorfromClass "/Game/Menu/Blueprints/MenuVRPawn.MenuVRPawn_C" _returnvalue_3 "Undefined" 0 0))
      (Actor|DestroyActor (Game|Player|GetPlayerPawn 0))
      (Pawn|Possess (Game|GetPlayerController 0) _returnvalue_4))
    (:NewEnumerator1
      (bind _returnvalue_5 (Game|SpawnActorfromClass "/Game/Menu/Blueprints/MenuThirdPerson.MenuThirdPerson_C" _returnvalue_3 "Undefined" 0 0))
      (Actor|DestroyActor (Game|Player|GetPlayerPawn 0))
      (Pawn|Possess (Game|GetPlayerController 0) _returnvalue_5)))
  (bind _tranforminfront (CallFunction|MenuPlacementinFrontOfActor (Game|Player|GetPlayerPawn 0) 65.0 0.2 4e+01))
  (bind _returnvalue_6 (Game|SpawnActorfromClass "/Game/Menu/Blueprints/VRActors/StartMenuActor.StartMenuActor_C" _tranforminfront "Undefined" 0 0))
  (Transformation|AttachActorToActor _returnvalue_6 (Game|Player|GetPlayerPawn 0) "None" "KeepWorld" "KeepWorld" "KeepWorld" false)
  (bind _aswb_menu (Utilities|Casting|CastToWB_Menu (UserInterface|GetUserWidgetObject (Variables|/Game/Menu/Blueprints/VRActors/StartMenuActor.StartMenuActor_C|GetWidget _returnvalue_6))))
  (Variables|Default|SetStartMenu _aswb_menu))

(fn ConstructionScript)