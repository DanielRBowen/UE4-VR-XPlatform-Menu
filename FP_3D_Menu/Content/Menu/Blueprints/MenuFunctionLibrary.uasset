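; Blueprint function library for VR menus that computes a transform to place a 3D menu in front of an actor.
; MenuPlacementInFrontOfActor combines headset yaw with the actor's root rotation flipped about 180 degrees, so the menu faces back toward the player.
; It offsets from the actor's location along the view yaw by the given distance, ignoring headset pitch and roll.
; Player height raises the result, and a uniform menu scale is applied.
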(fn MenuPlacementinFrontOfActor
  (params (spawningActor :type Actor%20Object%20Reference) (spawnDistanceFromActor :type Float%20%28single-precision%29) (3DMenuScale :type Float%20%28single-precision%29) (playerHeight :type Float%20%28single-precision%29))
  (bind _returnvalue (Transformation|GetActorLocation spawningActor))
  (bind _devicerotation (Class|HeadMountedDisplayFunctionLibrary|GetOrientationandPosition))
  (bind _rootcomponent (Variables|/Script/Engine.Actor|GetRootComponent spawningActor))
  (bind _returnvalue_2 (Transformation|GetWorldRotation _rootcomponent))
  (bind _yaw (Math|Rotator|BreakRotator _devicerotation))
  (bind _returnvalue_3 (* -1 spawnDistanceFromActor))
  (bind _returnvalue_4 (Math|Rotator|MakeRotator 0.0 0.0 _yaw))
  (bind (_roll _pitch _yaw_2) (Math|Rotator|BreakRotator _returnvalue_2))
  (bind _returnvalue_5 (Math|Vector|GetForwardVector _returnvalue_4))
  (bind _returnvalue_6 (+ _yaw_2 -179.999786))
  (bind _returnvalue_7 (Math|Rotator|MakeRotator _roll _pitch _returnvalue_6))
  (bind _returnvalue_8 (Math|Vector|RotateVector _returnvalue_5 _returnvalue_7))
  (bind _returnvalue_9 (* _returnvalue_8 _returnvalue_3))
  (bind _returnvalue_10 (+ _returnvalue _returnvalue_9))
  (bind (_x _y _z) (Math|Vector|BreakVector _returnvalue_10))
  (return (Math|Transform|MakeTransform (Math|Vector|MakeVector _x _y (+ _z playerHeight)) (Math|Rotator|CombineRotators _returnvalue_4 _returnvalue_7) (Math|Conversions|ToVector(Float) 3DMenuScale))))