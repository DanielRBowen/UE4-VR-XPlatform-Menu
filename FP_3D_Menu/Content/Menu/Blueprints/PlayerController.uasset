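; Player controller for the menu game mode that routes menu input to whichever menu is active.
; On BeginPlay it takes the start menu from MenuMode and binds to its new-active-menu event so the active menu reference can be swapped.
; Directional actions send navigation requests to the active menu and Okay presses its selected button.
; Escape quits the game.
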(event Custom|SetNewMenu
  (params (newMenu :type WB%20Menu%20Object%20Reference))
  (Variables|Default|SetActiveMenu newMenu))

(event EventBeginPlay
  (bind _asmenu_mode (Utilities|Casting|CastToMenuMode (Game|GetGameMode)))
  (bind _output_get (Variables|Default|SetActiveMenu (Variables|/Game/Menu/Blueprints/MenuMode.MenuMode_C|GetStartMenu _asmenu_mode)))
  (EventDispatchers|BindEventtoNewActiveMenuSet _output_get (EventDispatchers|CreateEvent :!event Custom|SetNewMenu)))

(event Input|ActionEvents|InputActionMenuUp
  (params (Key :type Key%20Structure))
  (:Pressed
    (Default|ReceiveNavigationRequest (Variables|Default|GetActiveMenu) "NewEnumerator2")))

(event Input|ActionEvents|InputActionMenuRight
  (params (Key :type Key%20Structure))
  (:Pressed
    (Default|ReceiveNavigationRequest (Variables|Default|GetActiveMenu) "NewEnumerator1")))

(event Input|ActionEvents|InputActionMenuDown
  (params (Key :type Key%20Structure))
  (:Pressed
    (Default|ReceiveNavigationRequest (Variables|Default|GetActiveMenu) "NewEnumerator3")))

(event Input|ActionEvents|InputActionMenuLeft
  (params (Key :type Key%20Structure))
  (:Pressed
    (Default|ReceiveNavigationRequest (Variables|Default|GetActiveMenu) "NewEnumerator0")))

(event Input|ActionEvents|InputActionOkay
  (params (Key :type Key%20Structure))
  (:Pressed
    (Default|PressSelectedButton (Variables|Default|GetActiveMenu))))

(event Input|KeyboardEvents|Escape
  (params (Key :type Key%20Structure))
  (:Pressed
    (Game|QuitGame 0 "Quit" false)))

(fn ConstructionScript)